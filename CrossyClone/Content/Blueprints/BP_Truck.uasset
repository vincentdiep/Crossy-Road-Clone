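; BP_Truck is a moving vehicle hazard that kills the player's chicken on contact.
; On BeginPlay it randomly picks one of the two truck meshes from a six-mesh vehicle list.
; Tick moves the mesh along its local Y axis at TruckSpeed.
; Overlapping the collision box applies a squashing transform to BP_Player's chicken mesh and sets IsDead.
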(event OnComponentBeginOverlap(TruckColBox)
  (params (OverlappedComponent :type Primitive%20Component%20Object%20Reference) (OtherActor :type Actor%20Object%20Reference) (OtherComp :type Primitive%20Component%20Object%20Reference) (OtherBodyIndex :type Integer) (bFromSweep :type Boolean) (SweepResult :type Hit%20Result%20Structure%20%28by%20ref%29))
  (bind _asbp_player (Utilities|Casting|CastToBP_Player OtherActor))
  (Class|SceneComponent|AddLocalTransform (Variables|/Game/Blueprints/BP_Player.BP_Player_C|GetChickenMesh _asbp_player) (Math|Transform|MakeTransform "0, 0, 0" "0, 0, 0" "1,1,0.001000") false false)
  (Variables|/Game/Blueprints/BP_Player.BP_Player_C|SetIsDead _asbp_player true))

(event EventBeginPlay
  (CallFunction|RandomizeTruck))

(event Collision|EventActorBeginOverlap
  (params (OtherActor :type Actor%20Object%20Reference)))

(event EventTick
  (params (DeltaSeconds :type Float%20%28single-precision%29))
  (Transformation|AddLocalOffset (Variables|Default|GetTruckMesh) (Math|Vector|MakeVector 0.0 (* DeltaSeconds (Variables|Default|GetTruckSpeed)) 0.0) false false))

(fn ConstructionScript)

(fn RandomizeTruck
  (Components|StaticMesh|SetStaticMesh (Variables|Default|GetTruckMesh) (Utilities|Select :Index (Math|Random|RandomIntegerinRange 4 5) :Option%200 "/Game/Vehicles/long_green_car.long_green_car" :Option%201 "/Game/Vehicles/purple_car.purple_car" :Option%202 "/Game/Vehicles/orange_car.orange_car" :Option%203 "/Game/Vehicles/police_car.police_car" :Option%204 "/Game/Vehicles/csuf_truck.csuf_truck" :Option%205 "/Game/Vehicles/oil_truck.oil_truck")))