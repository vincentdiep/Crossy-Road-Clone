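; Player character for a hopping chicken, with jump input on forward/backward and left/right that is blocked when dead.
; Each hop calls Jump, then launches along X or Y by axis sign, capped by a counter reset on landing or hit.
; WASD keys snap the chicken mesh's yaw relative to the actor.
; Tick moves Scene along the actor's X with clamped Y and zero Z; the chicken spawn-and-attach logic is unconnected.
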(event Custom|CustomEvent
  (params (Hit :type Hit%20Result%20Structure%20%28by%20ref%29))
  ;[1 1 1] Jumping
  (Variables|Default|SetJumpCounter 0))

(event EventBeginPlay)

(event Collision|EventActorBeginOverlap
  (params (OtherActor :type Actor%20Object%20Reference)))

(event EventOnLanded
  (params (Hit :type Hit%20Result%20Structure%20%28by%20ref%29))
  ;[1 1 1] Jumping
  (Variables|Default|SetJumpCounter 0))

(event EventTick
  (params (DeltaSeconds :type Float%20%28single-precision%29))
  (bind _returnvalue (Transformation|GetActorLocation))
  (if (not (Variables|Default|GetIsDead))
    (Transformation|SetWorldLocation (Variables|Default|GetScene) (Math|Vector|MakeVector (.x _returnvalue) (Math|Float|Clamp(Float) (.y _returnvalue)) 0.0) true false)))

(event Input|ActionEvents|InputActionJumpForward/Backward
  (params (Key :type Key%20Structure :default "None"))
  ;[1 1 1] Jumping
  (:Pressed
    (if (not (Variables|Default|GetIsDead))
      (if (< (Variables|Default|GetJumpCounter) (Variables|Default|GetMaxJumps))
        (Variables|Default|SetJumpCounter (+ (Variables|Default|GetJumpCounter) 1))
        (Character|Jump)
        (Utilities|FlowControl|Delay 0.1)
        (Character|LaunchCharacter (Math|Vector|MakeVector (* (/ (stale Input|AxisEvents|InputAxisMoveForward/Backward AxisValue) (Math|Float|Absolute(Float) (stale Input|AxisEvents|InputAxisMoveForward/Backward AxisValue))) -1e+02) 0.0 0.0) false false))))
  (:Released
    (Character|StopJumping)))

(event Input|ActionEvents|InputActionJumpLeft/Right
  (params (Key :type Key%20Structure :default "None"))
  ;[1 1 1] Jumping
  (:Pressed
    (if (not (Variables|Default|GetIsDead))
      (if (< (Variables|Default|GetJumpCounter) (Variables|Default|GetMaxJumps))
        (Variables|Default|SetJumpCounter (+ (Variables|Default|GetJumpCounter) 1))
        (Character|Jump)
        (Utilities|FlowControl|Delay 0.1)
        (Character|LaunchCharacter (Math|Vector|MakeVector 0.0 (* (/ (stale Input|AxisEvents|InputAxisMoveRight/Left AxisValue) (Math|Float|Absolute(Float) (stale Input|AxisEvents|InputAxisMoveRight/Left AxisValue))) -1e+02) 0.0) false false))))
  (:Released
    (Character|StopJumping)))

(event Input|AxisEvents|InputAxisMoveRight/Left
  (params (AxisValue :type Float%20%28single-precision%29))
  ;[1 1 1] Jumping
)

(event Input|AxisEvents|InputAxisMoveForward/Backward
  (params (AxisValue :type Float%20%28single-precision%29))
  ;[1 1 1] Jumping
)

(event Input|KeyboardEvents|D
  (params (Key :type Key%20Structure :default "None"))
  (:Pressed
    (Utilities|FlowControl|DoOnce false :!label _label
      (:Completed
        (Transformation|SetWorldRotation (Variables|Default|GetChickenMesh) (Math|Rotator|MakeRotator 0.0 0.0 (+ (.yaw (Transformation|GetActorRotation)) -1.8e+02)) false false))))
  (:Released
    (goto _label Reset)))

(event Input|KeyboardEvents|A
  (params (Key :type Key%20Structure :default "None"))
  (:Pressed
    (Utilities|FlowControl|DoOnce false :!label _label
      (:Completed
        (Transformation|SetWorldRotation (Variables|Default|GetChickenMesh) (Math|Rotator|MakeRotator 0.0 0.0 (+ (.yaw (Transformation|GetActorRotation)) 0.0)) false false))))
  (:Released
    (goto _label Reset)))

(event Input|KeyboardEvents|W
  (params (Key :type Key%20Structure :default "None"))
  (:Pressed
    (Utilities|FlowControl|DoOnce false :!label _label
      (:Completed
        (Transformation|SetWorldRotation (Variables|Default|GetChickenMesh) (Math|Rotator|MakeRotator 0.0 0.0 (+ (.yaw (Transformation|GetActorRotation)) 9e+01)) false false))))
  (:Released
    (goto _label Reset)))

(event Input|KeyboardEvents|S
  (params (Key :type Key%20Structure :default "None"))
  (:Pressed
    (Utilities|FlowControl|DoOnce false :!label _label
      (:Completed
        (Transformation|SetWorldRotation (Variables|Default|GetChickenMesh) (Math|Rotator|MakeRotator 0.0 0.0 (+ (.yaw (Transformation|GetActorRotation)) -9e+01)) false false))))
  (:Released
    (goto _label Reset)))

(fn ConstructionScript)