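; Three-lane road segment that spawns car and truck traffic and chains into the next segment.
; After a random delay, BeginPlay spawns initial vehicles, then makes one follow-up pass gated by randomized Y gaps from the newest car and truck.
; A player entering the trigger zone has RoadSpawner spawn another road and destroys this one.
; Cars and trucks are destroyed when they leave their respective trigger zones.
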(event OnComponentBeginOverlap(TriggerZone)
  (params (OverlappedComponent :type Primitive%20Component%20Object%20Reference) (OtherActor :type Actor%20Object%20Reference) (OtherComp :type Primitive%20Component%20Object%20Reference) (OtherBodyIndex :type Integer) (bFromSweep :type Boolean) (SweepResult :type Hit%20Result%20Structure%20%28by%20ref%29))
  (Utilities|Casting|CastToBP_Player OtherActor)
  (Default|SpawnRoadatSpawnPoint (Variables|Default|GetRoadSpawner))
  (Actor|DestroyActor))

(event OnComponentEndOverlap(CarTriggerZone)
  (params (OverlappedComponent :type Primitive%20Component%20Object%20Reference) (OtherActor :type Actor%20Object%20Reference) (OtherComp :type Primitive%20Component%20Object%20Reference) (OtherBodyIndex :type Integer))
  (bind _asbp_car (Utilities|Casting|CastToBP_Car OtherActor))
  (Actor|DestroyActor _asbp_car))

(event OnComponentEndOverlap(TruckTriggerZone)
  (params (OverlappedComponent :type Primitive%20Component%20Object%20Reference) (OtherActor :type Actor%20Object%20Reference) (OtherComp :type Primitive%20Component%20Object%20Reference) (OtherBodyIndex :type Integer))
  (bind _asbp_truck (Utilities|Casting|CastToBP_Truck OtherActor))
  (Actor|DestroyActor _asbp_truck))

(event EventBeginPlay
  (bind _returnvalue (Math|Random|RandomFloatinRange 7.0 1e+01))
  (Utilities|FlowControl|Delay (Math|Random|RandomFloatinRange 0.5 6.0))
  (CallFunction|SpawnInitialCars)
  (CallFunction|SpawnInitialTrucks)
  (if (> (Math|Float|Absolute(Float) (- (.y (Transformation|GetWorldLocation (Variables|/Game/Blueprints/BP_Car.BP_Car_C|GetCarMesh (Variables|Default|GetNewestCar)))) (.y (Transformation|GetWorldLocation (Variables|Default|GetCarSpawnPoint))))) (Math|Conversions|ToFloat(Integer) (Math|Random|RandomIntegerinRange 50 100)))
    (CallFunction|SpawnCar (Transformation|GetWorldLocation (Variables|Default|GetCarSpawnPoint)))
    (Utilities|FlowControl|Delay _returnvalue)
    (if (> (Math|Float|Absolute(Float) (- (.y (Transformation|GetWorldLocation (Variables|/Game/Blueprints/BP_Truck.BP_Truck_C|GetTruckMesh (Variables|Default|GetNewestTruck)))) (.y (Transformation|GetWorldLocation (Variables|Default|GetTruckSpawnPoint))))) (Math|Conversions|ToFloat(Integer) (Math|Random|RandomIntegerinRange 100 200)))
      (CallFunction|SpawnTruck (Transformation|GetWorldLocation (Variables|Default|GetTruckSpawnPoint)))
      (Utilities|FlowControl|Delay _returnvalue))))

(event Collision|EventActorBeginOverlap
  (params (OtherActor :type Actor%20Object%20Reference)))

(event EventTick
  (params (DeltaSeconds :type Float%20%28single-precision%29)))

(fn ConstructionScript)

(fn SpawnCar
  (params (CarSpawnLocation :type Vector))
  (bind _returnvalue (Game|SpawnActorfromClass "/Game/Blueprints/BP_Car.BP_Car_C" (Math|Transform|MakeTransform CarSpawnLocation "0, 0, 0" "1,1,1") "Undefined" 0 0))
  (bind _output_get (Variables|Default|SetNewestCar _returnvalue))
  (Variables|/Game/Blueprints/BP_Car.BP_Car_C|SetCarSpawner _output_get self))

(fn SpawnCaratCarSpawn
  (if (> (Math|Float|Absolute(Float) (- (.y (Transformation|GetWorldLocation (Variables|/Game/Blueprints/BP_Car.BP_Car_C|GetCarMesh (Variables|Default|GetNewestCar)))) (.y (Transformation|GetWorldLocation (Variables|Default|GetCarSpawnPoint))))) (Math|Conversions|ToFloat(Integer) (Math|Random|RandomIntegerinRange 200 800)))
    (CallFunction|SpawnCar (Transformation|GetWorldLocation (Variables|Default|GetCarSpawnPoint)))))

(fn SpawnInitialCars
  (for _index (range 0 1)
    (Utilities|IsValid (Variables|Default|GetNewestCar)
      (:Is%20Valid
        (CallFunction|SpawnCaratCarSpawn))
      (:Is%20Not%20Valid
        (CallFunction|SpawnCar (Transformation|GetWorldLocation (Variables|Default|GetCarSpawnPoint)))))))

(fn SpawnTruck
  (params (TruckSpawnLocation :type Vector))
  (bind _returnvalue (Game|SpawnActorfromClass "/Game/Blueprints/BP_Truck.BP_Truck_C" (Math|Transform|MakeTransform TruckSpawnLocation "0, 0, 0" "1,1,1") "Undefined" 0 0))
  (bind _output_get (Variables|Default|SetNewestTruck _returnvalue))
  (Variables|/Game/Blueprints/BP_Truck.BP_Truck_C|SetTruckSpawner _output_get self))

(fn SpawnTruckatTruckSpawn
  (if (> (Math|Float|Absolute(Float) (- (.y (Transformation|GetWorldLocation (Variables|/Game/Blueprints/BP_Truck.BP_Truck_C|GetTruckMesh (Variables|Default|GetNewestTruck)))) (.y (Transformation|GetWorldLocation (Variables|Default|GetTruckSpawnPoint))))) (Math|Conversions|ToFloat(Integer) (Math|Random|RandomIntegerinRange 300 400)))
    (CallFunction|SpawnTruck (Transformation|GetWorldLocation (Variables|Default|GetTruckSpawnPoint)))))

(fn SpawnInitialTrucks
  (for _index (range 0 1)
    (Utilities|IsValid (Variables|Default|GetNewestTruck)
      (:Is%20Valid
        (CallFunction|SpawnTruckatTruckSpawn))
      (:Is%20Not%20Valid
        (CallFunction|SpawnTruck (Transformation|GetWorldLocation (Variables|Default|GetTruckSpawnPoint)))))))