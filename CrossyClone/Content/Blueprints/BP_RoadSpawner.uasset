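; Spawner actor that builds a chain of three-lane road segments, starting just below the player pawn on BeginPlay.
; The first segment uses the pawn's location, and each later one spawns at the newest segment's SpawnPoint.
; Each spawned road becomes NewestRoad and receives a reference to the spawner.
; A separate SpawnGrass function spawns grass at a given location but is not called within this Blueprint.
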(event EventBeginPlay
  (CallFunction|SpawnInitialRoads))

(event Collision|EventActorBeginOverlap
  (params (OtherActor :type Actor%20Object%20Reference)))

(event EventTick
  (params (DeltaSeconds :type Float%20%28single-precision%29)))

(fn ConstructionScript)

(fn SpawnRoad
  (params (SpawnLocation :type Vector))
  (bind _returnvalue (Game|SpawnActorfromClass "/Game/Blueprints/BP_3LaneRoad.BP_3LaneRoad_C" (Math|Transform|MakeTransform SpawnLocation "0, 0, 0" "1,1,1") "Undefined" 0 0))
  (bind _output_get (Variables|Default|SetNewestRoad _returnvalue))
  (Variables|/Game/Blueprints/BP_3LaneRoad.BP_3LaneRoad_C|SetRoadSpawner _output_get self))

(fn SpawnRoadatSpawnPoint
  (CallFunction|SpawnRoad (Transformation|GetWorldLocation (Variables|/Game/Blueprints/BP_3LaneRoad.BP_3LaneRoad_C|GetSpawnPoint (Variables|Default|GetNewestRoad)))))

(fn SpawnInitialRoads
  (bind _returnvalue (Game|Player|GetPlayerPawn 0))
  (bind _returnvalue_2 (Transformation|GetActorLocation _returnvalue))
  (for _index (range 0 10)
    (Utilities|IsValid (Variables|Default|GetNewestRoad)
      (:Is%20Valid
        (CallFunction|SpawnRoadatSpawnPoint))
      (:Is%20Not%20Valid
        (CallFunction|SpawnRoad (Math|Vector|MakeVector (.x _returnvalue_2) (.y _returnvalue_2) (- (.z _returnvalue_2) 5.0)))))))

(fn SpawnGrass
  (params (SpawnLocation :type Vector))
  (Game|SpawnActorfromClass "/Game/Blueprints/BP_Grass.BP_Grass_C" (Math|Transform|MakeTransform SpawnLocation "0, 0, 0" "1,1,1") "Undefined" 0 0))